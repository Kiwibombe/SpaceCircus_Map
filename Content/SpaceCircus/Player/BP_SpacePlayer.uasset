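; Player character Blueprint for Space Circus that adds a fuel-limited jetpack.
; Enhanced Input drives IA_Jetpack, launching the character upward by a delta-time-scaled velocity while draining charge.
; Tick timestamps Walking and Falling states, then refills charge at the drain rate once a delay has passed since last falling.
; BeginPlay creates the user widget, whose progress bar updates on every charge change.
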(event Input|EnhancedActionEvents|EnhancedInputActionIA_Jetpack
  (params (ActionValue :type Boolean) (ElapsedSeconds :type Float%20%28double-precision%29) (TriggeredSeconds :type Float%20%28double-precision%29) (InputAction :type Input%20Action%20Object%20Reference :default "/Game/SpaceCircus/Player/Input/Actions/IA_Jetpack.IA_Jetpack"))
  ;[0.15 0.15 0.15 0.5] Jetpack
  (if (> (Variables|Jetpack|GetJetpackCharge) 0.0)
    (Character|LaunchCharacter (Math|Vector|MakeVector 0.0 0.0 (* (Utilities|Time|GetWorldDeltaSeconds) (Variables|Default|GetJetpackVelocitySecond))) false false)
    (Jetpack|DepleteJetpack (* (Variables|Jetpack|GetJetpackFuelCostSecond) (Utilities|Time|GetWorldDeltaSeconds)))))

(event EventBeginPlay
  (bind _returnvalue (Game|GetPlayerController 0))
  (bind _returnvalue_2 (PlayerController|LocalPlayerSubsystems|GetEnhancedInputLocalPlayerSubsystem _returnvalue))
  (|CallParentFunction)
  (Utilities|FlowControl|Sequence
    (:then_0
      (bind _returnvalue_3 (UserInterface|CreateWidget "/Game/SpaceCircus/Player/BP_UserWidget.BP_UserWidget_C" (Game|GetPlayerController 0)))
      (bind _output_get (Variables|Default|SetUI_Widget _returnvalue_3))
      (UserInterface|Viewport|AddtoViewport _output_get 0))
    (:then_1
      (Utilities|IsValid _returnvalue_2
        (:Is%20Valid
          (Input|AddMappingContext _returnvalue_2 "/Game/SpaceCircus/Player/Input/IMC_Jetpack.IMC_Jetpack" 1 "(bIgnoreAllPressedKeysUntilRelease=True,bForceImmediately=False,bNotifyUserSettings=False)"))))
    (:then_2
      (Variables|Jetpack|SetJetpackCharge (Variables|Jetpack|GetMaxJetpackCharge))
      (UI_Widget|NotifyWidgetJetpackCharge))))

(event Collision|EventActorBeginOverlap
  (params (OtherActor :type Actor%20Object%20Reference)))

(event EventTick
  (params (DeltaSeconds :type Float%20%28single-precision%29))
  (Utilities|FlowControl|Sequence
    (:then_0
      (CallFunction|IsonGround))
    (:then_1
      (if (>= (- (GameState|GetServerWorldTimeSeconds (Game|GetGameState)) (Variables|Default|GetLastAirTime)) (Variables|Jetpack|GetJetpackRechargeDelay))
        (Jetpack|RechargeJetpack (* (Variables|Jetpack|GetJetpackFuelCostSecond) (Utilities|Time|GetWorldDeltaSeconds)))))))

(fn ConstructionScript
  (|CallParentFunction))

(fn IsonGround
  ;[0.15 0.15 0.15 0.5] If on ground, update LastGroundTime variable with current world time (can be used to check air time)
  (switch Utilities|FlowControl|Switch|SwitchonEMovementMode (Variables|/Script/Engine.CharacterMovementComponent|GetMovementMode (Variables|Character|GetCharacterMovement))
    (:MOVE_Walking
      (Variables|Default|SetLastGroundTime (GameState|GetServerWorldTimeSeconds (Game|GetGameState))))
    (:MOVE_Falling
      (Variables|Default|SetLastAirTime (GameState|GetServerWorldTimeSeconds (Game|GetGameState))))))

(fn RechargeJetpack
  (params (Charge :type Float%20%28double-precision%29))
  (Variables|Jetpack|SetJetpackCharge (Math|Float|Min(Float) (+ (Variables|Jetpack|GetJetpackCharge) Charge) (Variables|Jetpack|GetMaxJetpackCharge)))
  (UI_Widget|NotifyWidgetJetpackCharge))

(fn DepleteJetpack
  (params (Depletion :type Float%20%28double-precision%29))
  (Variables|Jetpack|SetJetpackCharge (Math|Float|Max(Float) (- (Variables|Jetpack|GetJetpackCharge) Depletion) 0.0))
  (UI_Widget|NotifyWidgetJetpackCharge))

(fn NotifyWidgetJetpackCharge
  (Progress|SetPercent (Variables|/Game/SpaceCircus/Player/BP_UserWidget.BP_UserWidget_C|GetJetPackChargeProgess (Variables|Default|GetUI_Widget)) (/ (Variables|Jetpack|GetJetpackCharge) (Variables|Jetpack|GetMaxJetpackCharge))))