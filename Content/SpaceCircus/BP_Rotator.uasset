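; BP_Rotator is a Space Circus Blueprint that orbits a list of actors around a center point in the horizontal plane.
; Every Tick it loops over ObjectsToRotate and applies a 2D sine/cosine rotation about Center to each location, keeping Z, without sweeping.
; It also adds matching local yaw, so each actor turns with its orbit at DegreesPerSecond, scaled by delta time.
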(event EventBeginPlay)

(event Collision|EventActorBeginOverlap
  (params (OtherActor :type Actor%20Object%20Reference)))

(event EventTick
  (params (DeltaSeconds :type Float%20%28single-precision%29))
  (bind _center (Variables|Default|GetCenter))
  (bind _center_2 (Variables|Default|GetCenter))
  (Variables|Default|SetDelta%20Seconds DeltaSeconds)
  (for _array_element (Variables|Default|GetObjectsToRotate)
    (Transformation|SetActorLocation _array_element (Math|Vector|MakeVector (+ (- (* (- (.x (Transformation|GetActorLocation _array_element)) (.x _center_2)) (Math|Trig|Cos(Degrees) (* (Variables|Default|GetDegreesPerSecond) (Variables|Default|GetDelta%20Seconds)))) (* (- (.y (Transformation|GetActorLocation _array_element)) (.y _center_2)) (Math|Trig|Sin(Degrees) (* (Variables|Default|GetDegreesPerSecond) (Variables|Default|GetDelta%20Seconds))))) (.x _center)) (+ (.y _center) (+ (* (- (.x (Transformation|GetActorLocation _array_element)) (.x _center_2)) (Math|Trig|Sin(Degrees) (* (Variables|Default|GetDegreesPerSecond) (Variables|Default|GetDelta%20Seconds)))) (* (- (.y (Transformation|GetActorLocation _array_element)) (.y _center_2)) (Math|Trig|Cos(Degrees) (* (Variables|Default|GetDegreesPerSecond) (Variables|Default|GetDelta%20Seconds)))))) (.z (Transformation|GetActorLocation _array_element))) false false)
    (Transformation|AddActorLocalRotation _array_element (Math|Rotator|MakeRotator 0.0 0.0 (* (Variables|Default|GetDegreesPerSecond) (Variables|Default|GetDelta%20Seconds))) false false)))

(fn ConstructionScript)