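; Grenade launcher weapon component that fires a grenade projectile for the player.
; When the shoot input starts, it spawns a BP_GrenadeProjectile at the first-person camera's world location, with a transform built from location alone.
; It then passes its damage, explosion tuning and player reference to the new grenade through SetGrenadeValues.
; The component itself applies no aim direction, fire-rate limit or ammo check.
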(event Input|EnhancedActionEvents|EnhancedInputActionIA_Shoot
  (params (ActionValue :type Boolean) (ElapsedSeconds :type Float%20%28double-precision%29) (TriggeredSeconds :type Float%20%28double-precision%29) (InputAction :type Input%20Action%20Object%20Reference :default "/Game/SpaceCircus/Player/Input/Actions/IA_Shoot.IA_Shoot"))
  (:Started
    (bind _returnvalue (Game|SpawnActorfromClass "/Game/SpaceCircus/Weapon/GrenadeLauncher/BP_GrenadeProjectile.BP_GrenadeProjectile_C" (Math|Conversions|ToTransform(Vector) (Transformation|GetWorldLocation (Variables|/Game/FirstPerson/Blueprints/BP_FirstPersonCharacter.BP_FirstPersonCharacter_C|GetFirstPersonCamera (Variables|Default|GetSpacePlayerRef)))) "Undefined" "MultiplyWithRoot" 0 0))
    (Default|SetGrenadeValues _returnvalue (Variables|Damage|GetProjectileDamage) (Variables|Damage|GetExplosionDamage) (Variables|Damage|GetExplosionFallOfStart) (Variables|Damage|GetExplosionRadius) (Variables|Default|GetSpacePlayerRef))))

(event EventBeginPlay
  (|CallParentFunction) ; This node is disabled and will not be called.\nDrag off pins to build functionality.
)

(event EventTick
  (params (DeltaSeconds :type Float%20%28single-precision%29))
  (|CallParentFunction DeltaSeconds) ; This node is disabled and will not be called.\nDrag off pins to build functionality.
)