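; Grenade launcher projectile for SpaceCircus that explodes when it hits any actor other than the referenced space player.
; SetGrenadeValues stores the player reference along with damage, explosion damage, falloff and radius values.
; BeginPlay binds the actor hit event, which filters out that player and calls Explode.
; Explode is a placeholder that prints a debug string and destroys the actor without applying the stored damage values.
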(event Custom|OnActorHit_Event
  (params (SelfActor :type Actor%20Object%20Reference) (OtherActor :type Actor%20Object%20Reference) (NormalImpulse :type Vector) (Hit :type Hit%20Result%20Structure%20%28by%20ref%29))
  (if (not (== OtherActor (Variables|Default|GetSpacePlayerRef)))
    (CallFunction|Explode OtherActor)))

(event Custom|Explode
  (params (OtherActor :type Actor%20Object%20Reference))
  (Development|PrintString "BOOOOM")
  (Actor|DestroyActor))

(event Collision|EventActorBeginOverlap
  (params (OtherActor :type Actor%20Object%20Reference)))

(event EventTick
  (params (DeltaSeconds :type Float%20%28single-precision%29)))

(event EventBeginPlay
  (EventDispatchers|BindEventtoOnActorHit (delegate Custom|OnActorHit_Event)))

(fn ConstructionScript)

(fn SetGrenadeValues
  (params (Damage :type Float%20%28double-precision%29) (ExplosionDamage :type Float%20%28double-precision%29) (ExplosionFallOfStart :type Float%20%28double-precision%29) (ExplosionRadius :type Float%20%28double-precision%29) (SpacePlayerRef :type BP%20Space%20Player%20Object%20Reference))
  (Variables|Default|SetDamage Damage)
  (Variables|Default|SetExplosionDamage ExplosionDamage)
  (Variables|Default|SetExplosionFallOfStart ExplosionFallOfStart)
  (Variables|Default|SetExplosionRadius ExplosionRadius)
  (Variables|Default|SetSpacePlayerRef SpacePlayerRef)
  (return))