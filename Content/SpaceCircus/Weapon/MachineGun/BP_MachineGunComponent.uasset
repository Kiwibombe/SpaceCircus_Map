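; Machine gun component that fires a hitscan shot on the shoot input and damages any BP_SpacePlayer it hits.
; A debug-drawn Camera-channel line trace runs from the owning player's first-person camera, with random spread applied to its end point.
; Damage is full inside the first falloff distance, linearly interpolated between paired distance and multiplier array entries, and held at the last multiplier beyond them.
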(event Input|EnhancedActionEvents|EnhancedInputActionIA_Shoot
  (params (ActionValue :type Boolean) (ElapsedSeconds :type Float%20%28double-precision%29) (TriggeredSeconds :type Float%20%28double-precision%29) (InputAction :type Input%20Action%20Object%20Reference :default "/Game/SpaceCircus/Player/Input/Actions/IA_Shoot.IA_Shoot"))
  (bind _spaceplayerref (Variables|Default|GetSpacePlayerRef))
  (bind _maxspreadradius (Variables|Spread|GetMaxSpreadRadius))
  (bind _maxfallofdamagereduction (Variables|Damage|GetMaxFallOfDamageReduction))
  (bind _fallofdistancedistances (Variables|Damage|GetFallOfDistanceDistances))
  (bind _returnvalue (* _maxspreadradius -1.0))
  (bind _firstpersoncamera (Variables|/Game/FirstPerson/Blueprints/BP_FirstPersonCharacter.BP_FirstPersonCharacter_C|GetFirstPersonCamera _spaceplayerref))
  (bind _returnvalue_2 (Transformation|GetWorldLocation _firstpersoncamera))
  (bind _outhit (Collision|LineTraceByChannel _returnvalue_2 (+ (+ _returnvalue_2 (* (Math|Vector|GetForwardVector (Variables|/Game/FirstPerson/Blueprints/BP_FirstPersonCharacter.BP_FirstPersonCharacter_C|GetFirstPersonCamera (Variables|Default|GetSpacePlayerRef))) 1e+04)) (Math|Vector|MakeVector (Math|Random|RandomFloatinRange _returnvalue (Variables|Spread|GetMaxSpreadRadius)) (Math|Random|RandomFloatinRange _returnvalue (Variables|Spread|GetMaxSpreadRadius)) (Math|Random|RandomFloatinRange _returnvalue (Variables|Spread|GetMaxSpreadRadius)))) "TraceTypeQuery2" false 0 "ForDuration"))
  (Variables|Default|SetOut%20Hit%20Distance (.distance _outhit))
  (bind _asbp_space_player (Utilities|Casting|CastToBP_SpacePlayer (.hitactor _outhit)))
  (Variables|Default|SetHit%20Player _asbp_space_player)
  (Variables|Default|SetHitDone false)
  (if (< (Variables|Default|GetOut%20Hit%20Distance) (Utilities|Array|Get(acopy) (Variables|Damage|GetFallOfDistanceDistances)))
    (Default|ReceiveDamage (Variables|Default|GetHit%20Player) (Variables|Damage|GetDamage) 0 0 "/Script/Engine.DamageType")
    (else
      (bind _index (Utilities|FlowControl|ForLoopwithBreak 1 (- (Utilities|Array|Length (Variables|Damage|GetFallOfDistanceDistances)) 1) :!label _label)
        (:LoopBody
          (if (<= (Variables|Default|GetOut%20Hit%20Distance) (Utilities|Array|Get(acopy) (Variables|Damage|GetFallOfDistanceDistances) _index))
            (Default|ReceiveDamage (Variables|Default|GetHit%20Player) (* (Variables|Damage|GetDamage) (- (Utilities|Array|Get(acopy) (Variables|Damage|GetMaxFallOfDamageReduction) (- _index 1)) (* (/ (- (Variables|Default|GetOut%20Hit%20Distance) (Utilities|Array|Get(acopy) _fallofdistancedistances (- _index 1))) (- (Utilities|Array|Get(acopy) _fallofdistancedistances _index) (Utilities|Array|Get(acopy) _fallofdistancedistances (- _index 1)))) (- (Utilities|Array|Get(acopy) (Variables|Damage|GetMaxFallOfDamageReduction) (- _index 1)) (Utilities|Array|Get(acopy) (Variables|Damage|GetMaxFallOfDamageReduction) _index))))) 0 0 "/Script/Engine.DamageType")
            (Variables|Default|SetHitDone true)
            (goto _label Break)))
        (:Completed
          (if (not (Variables|Default|GetHitDone))
            (Default|ReceiveDamage (Variables|Default|GetHit%20Player) (* (Variables|Damage|GetDamage) (Utilities|Array|Get(acopy) _maxfallofdamagereduction (- (Utilities|Array|Length _maxfallofdamagereduction) 1))))))))))

(event EventBeginPlay
  (|CallParentFunction) ; This node is disabled and will not be called.\nDrag off pins to build functionality.
)

(event EventTick
  (params (DeltaSeconds :type Float%20%28single-precision%29))
  (|CallParentFunction DeltaSeconds) ; This node is disabled and will not be called.\nDrag off pins to build functionality.
)