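; Weapon pickup actor that swaps the weapon held by an overlapping BP_SpacePlayer and respawns after a delay.
; On sphere overlap it removes the first weapon component on the first-person mesh, hides itself and calls CreateComponent, an empty function here, presumably for child overrides.
; Tick counts down DisableDuration to show it again.
; Hiding leaves collision on and overlap never checks Enabled, so a hidden pickup still triggers.
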(event OnComponentBeginOverlap(Sphere)
  (params (OverlappedComponent :type Primitive%20Component%20Object%20Reference) (OtherActor :type Actor%20Object%20Reference) (OtherComp :type Primitive%20Component%20Object%20Reference) (OtherBodyIndex :type Integer) (bFromSweep :type Boolean) (SweepResult :type Hit%20Result%20Structure%20%28by%20ref%29))
  (bind _asbp_space_player (Utilities|Casting|CastToBP_SpacePlayer OtherActor))
  (bind _output_get (Variables|Default|SetSpacePlayerRef _asbp_space_player))
  ;[0.15 0.15 0.15 0.5] Check if player has a weapon component already
  (Variables|Default|SetbPlayerHasWeapon false)
  (bind _array_element (Utilities|Array|ForEachLoopwithBreak (Components|GetChildrenComponents (Variables|/Game/FirstPerson/Blueprints/BP_FirstPersonCharacter.BP_FirstPersonCharacter_C|GetFirstPersonMesh _output_get) false) :!label _label)
    (:LoopBody
      (bind _asbp_weapon_component (Utilities|Casting|CastToBP_WeaponComponent _array_element))
      (Default|RemoveComponent _asbp_weapon_component)
      (Variables|Default|SetbPlayerHasWeapon false)
      (goto _label Break))
    (:Completed
      (if (not (Variables|Default|GetbPlayerHasWeapon))
        (CallFunction|EnablePickup false)
        (CallFunction|CreateComponent _output_get)))))

(event EventBeginPlay
  (CallFunction|EnablePickup true))

(event Collision|EventActorBeginOverlap
  (params (OtherActor :type Actor%20Object%20Reference)))

(event EventTick
  (params (DeltaSeconds :type Float%20%28single-precision%29))
  (if (not (Variables|Default|GetbEnabled))
    (bind _output_get (Variables|Default|SetDisableTimer (- (Variables|Default|GetDisableTimer) DeltaSeconds)))
    (if (<= _output_get 0.0)
      (CallFunction|EnablePickup true))))

(fn ConstructionScript)

(fn CreateComponent
  (params (SpacePlayerRef :type BP%20Space%20Player%20Object%20Reference))
  (return))

(fn EnablePickup
  (params (Enable :type Boolean))
  (Variables|Default|SetbEnabled Enable)
  (Rendering|SetActorHiddenInGame (not Enable))
  (if (not (Variables|Default|GetbEnabled))
    (Variables|Default|SetDisableTimer (Variables|Default|GetDisableDuration))))